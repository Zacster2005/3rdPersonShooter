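; BPC_Attack_System is a character component that runs a four-step melee combo of sword attacks and a kick.
; IA_Attack calls SwordAttack when CanAttack is set, which either buffers input in SaveAttack while IsAttacking or plays the montage selected by AttackIndex.
; Each step advances the index behind a DoOnce gate.
; SwordAttackCombo, not called within this graph, consumes buffered input to continue the chain or resets it through StopCombo.
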(event Custom|SwordAttack
  ;[1 1 1] Sword Attack
  (if (Variables|Default|Getis%20Attacking?)
    (Variables|Default|SetSaveAttack? true)
    (else
      (Variables|Default|SetSaveAttack? false)
      (switch int (Variables|Default|GetAttack%20Index)
        (:0
          (CallFunction|Attack1))
        (:1
          (CallFunction|Attack2))
        (:2
          (CallFunction|Attack3))
        (:3
          (CallFunction|Attack4))))))

(event Custom|Sword%20Attack%20Combo
  ;[1 1 1] Sword Combo
  (if (Variables|Default|GetSaveAttack?)
    (Variables|Default|SetSaveAttack? false)
    (switch int (Variables|Default|GetAttack%20Index)
      (:0
        (CallFunction|Attack1))
      (:1
        (CallFunction|Attack2))
      (:2
        (CallFunction|Attack3))
      (:3
        (CallFunction|Attack4)))
    (else
      (CallFunction|StopCombo))))

(event Custom|Stop%20Combo
  ;[1 1 1] Stop Combo
  (Variables|Default|Setis%20Attacking? false)
  (Variables|Default|SetAttack%20Index 0))

(event Custom|Attack%204
  ;[1 1 1] Attack 1
  (Utilities|FlowControl|DoOnce false :!label _label
    (:Completed
      (Utilities|FlowControl|Delay 0.1)
      (Animation|Montage|PlayMontage 0 "/Game/Characters/RPG_Character/Animations/Sword_Attacks/Attack3_Montage.Attack3_Montage"
        (:then
          (Variables|Default|SetAttack%20Index 4)
          (goto _label Reset))))))

(event Custom|Attack%201
  ;[1 1 1] Attack 1
  (Utilities|FlowControl|DoOnce false :!label _label
    (:Completed
      (Utilities|FlowControl|Delay 0.1)
      (Animation|Montage|PlayMontage 0 "/Game/Characters/RPG_Character/Animations/Sword_Attacks/Attack1_Montage.Attack1_Montage"
        (:then
          (Variables|Default|SetAttack%20Index 1)
          (goto _label Reset))))))

(event Custom|Attack%202
  ;[1 1 1] Attack 1
  (Utilities|FlowControl|DoOnce false :!label _label
    (:Completed
      (Utilities|FlowControl|Delay 0.1)
      (Animation|Montage|PlayMontage 0 "/Game/Characters/RPG_Character/Animations/Sword_Attacks/Attack2_Montage.Attack2_Montage"
        (:then
          (Variables|Default|SetAttack%20Index 2)
          (goto _label Reset))))))

(event Custom|Attack3
  ;[1 1 1] Attack 1
  (Utilities|FlowControl|DoOnce false :!label _label
    (:Completed
      (Utilities|FlowControl|Delay 0.1)
      (Animation|Montage|PlayMontage 0 "/Game/Characters/RPG_Character/Animations/Sword_Attacks/Kick_Montage.Kick_Montage"
        (:then
          (Variables|Default|SetAttack%20Index 3)
          (goto _label Reset))))))

(event Input|EnhancedActionEvents|EnhancedInputActionIA_Attack
  (params (ActionValue :type Boolean) (ElapsedSeconds :type Float%20%28double-precision%29) (TriggeredSeconds :type Float%20%28double-precision%29) (InputAction :type Input%20Action%20Object%20Reference :default "/Game/ThirdPerson/Input/Actions/IA_Attack.IA_Attack"))
  ;[1 1 1] Input
  (:Started
    (if (Variables|Default|GetCan%20Attack?)
      (CallFunction|SwordAttack))))

(event EventBeginPlay
  (bind _asbp_third_person_character (Utilities|Casting|CastToBP_ThirdPersonCharacter (Components|GetOwner)))
  (Variables|Default|SetCharacter%20Mesh (Variables|/Script/Engine.Character|GetMesh _asbp_third_person_character)))